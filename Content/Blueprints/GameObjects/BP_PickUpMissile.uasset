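; BP_PickUpMissile is a pickup that gives the first-person character missile ammo.
; When the character overlaps its capsule, it adds one to the projectile count if the weapon is already Missile, printing the new total.
; Otherwise it switches the character's weapon type to Missile with a count of one.
; The pickup then destroys itself.
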(event OnComponentBeginOverlap(Capsule)
  (params (OverlappedComponent :type Primitive%20Component%20Object%20Reference) (OtherActor :type Actor%20Object%20Reference) (OtherComp :type Primitive%20Component%20Object%20Reference) (OtherBodyIndex :type Integer) (bFromSweep :type Boolean) (SweepResult :type Hit%20Result%20Structure%20%28by%20ref%29))
  (bind _asbp_first_person_character (Utilities|Casting|CastToBP_FirstPersonCharacter OtherActor))
  (if (Utilities|Enum|Equal(Enum) (Variables|/Game/FirstPerson/Blueprints/BP_FirstPersonCharacter.BP_FirstPersonCharacter_C|GetWeaponType _asbp_first_person_character) "Missile")
    (bind _result (Math|Integer|IncrementInt (Variables|/Game/FirstPerson/Blueprints/BP_FirstPersonCharacter.BP_FirstPersonCharacter_C|GetProjectileCount _asbp_first_person_character))
      (:%20%20
        (Variables|/Game/FirstPerson/Blueprints/BP_FirstPersonCharacter.BP_FirstPersonCharacter_C|SetProjectileCount _asbp_first_person_character _result)
        (Development|PrintString (Utilities|String|ToString(Integer) (Variables|/Game/FirstPerson/Blueprints/BP_FirstPersonCharacter.BP_FirstPersonCharacter_C|GetProjectileCount _asbp_first_person_character)))))
    (else
      (Variables|/Game/FirstPerson/Blueprints/BP_FirstPersonCharacter.BP_FirstPersonCharacter_C|SetWeaponType _asbp_first_person_character "Missile")
      (Variables|/Game/FirstPerson/Blueprints/BP_FirstPersonCharacter.BP_FirstPersonCharacter_C|SetProjectileCount _asbp_first_person_character 1)))
  (Actor|DestroyActor))

(fn ConstructionScript)