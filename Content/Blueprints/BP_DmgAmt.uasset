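; BP_DmgAmt is a floating damage number actor that shows an amount, drifts away from its spawn point and then disappears.
; On BeginPlay it passes DamageAmount to its W_DmgAmt widget component and stops early if that cast fails.
; The MoveT timeline then lerps the actor from its start location to a fixed diagonal, upward offset and destroys it when finished.
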(event EventBeginPlay
  (bind _asw_dmg_amt (Utilities|Casting|CastToW_DmgAmt (UserInterface|GetWidget (Variables|Default|GetWidget))))
  (Variables|/Game/HUD/W_DmgAmt.W_DmgAmt_C|SetDamageAmount _asw_dmg_amt (Variables|Default|GetDamage%20Amount))
  (bind _output_get (Variables|Default|SetStartLoc (Transformation|GetActorLocation)))
  (Variables|Default|SetEndLoc (+ _output_get "-25.000000,-25.000000,50.000000"))
  (bind _move_track (Timeline|Move%20T Play)
    (:Update
      (Transformation|SetActorLocation (Math|Vector|Lerp(Vector) (Variables|Default|GetStartLoc) (Variables|Default|GetEndLoc) _move_track) false false))
    (:Finished
      (Actor|DestroyActor))))

(fn ConstructionScript)